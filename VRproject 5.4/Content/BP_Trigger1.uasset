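; One-shot overlap trigger that advances a shared, staged escalation of a material effect, ending in a camera fade.
; Its first overlap increments the Triggers count on BP_GameManager and switches on it to play that stage's timeline.
; Early stages ease the material's Blend higher while lowering the minimum light value; the fifth oscillates Blend with a sine.
; The sixth eases Amplitude down and calls FadeCamera on the first-person character.
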(event `self.ReceiveBeginPlay`
  (bind _returnvalue (`GameplayStatics.GetActorOfClass` "/Game/BP_GameManager.BP_GameManager_C"))
  (set `self.GameManager` _returnvalue)
  (bind _returnvalue_2 (`GameplayStatics.GetActorOfClass` "/Game/FirstPerson/Blueprints/BP_FirstPersonCharacter.BP_FirstPersonCharacter_C"))
  (set `self.FirstPersonChar` _returnvalue_2))

(event `self.ReceiveActorBeginOverlap`
  (params (OtherActor :type "Actor Object Reference"))
  (bind _gamemanager (`self.GameManager`))
  (bind _firstpersonchar (`self.FirstPersonChar`))
  (`/Engine/EditorBlueprintResources/StandardMacros.DoOnce` false
    (:`Completed`
      (bind _output_get (set `/Game/BP_GameManager.Triggers` (+ (`/Game/BP_GameManager.Triggers` _gamemanager) 1.0) _gamemanager))
      (bind _returnvalue (`MaterialInstanceDynamic.K2_GetScalarParameterValue` (`/Game/BP_GameManager.MI` (`self.GameManager`)) "Blend"))
      (switch `int` (`KismetMathLibrary.FTrunc` _output_get)
        (:`1`
          (bind (_direction _alpha) (`Timeline|Transition` :!via `PlayFromStart`)
            (:`Update`
              (`MaterialInstanceDynamic.SetScalarParameterValue` (`/Game/BP_GameManager.MI` (`self.GameManager`)) "Blend" (`KismetMathLibrary.FInterpEaseInOut` _returnvalue 0.5 _alpha 2.0))
              (set `/Game/BP_GameManager.LIghtMinValue` 0.8 (`self.GameManager`)))))
        (:`2`
          (bind (_direction_2 _alpha_2) (`Timeline|Timeline` :!via `PlayFromStart`)
            (:`Update`
              (`MaterialInstanceDynamic.SetScalarParameterValue` (`/Game/BP_GameManager.MI` (`self.GameManager`)) "Blend" (`KismetMathLibrary.FInterpEaseInOut` _returnvalue 1.0 _alpha_2 2.0))
              (set `/Game/BP_GameManager.LIghtMinValue` 0.6 (`self.GameManager`)))))
        (:`3`
          (bind (_direction_3 _alpha_3) (`Timeline|Timeline_0` :!via `PlayFromStart`)
            (:`Update`
              (`MaterialInstanceDynamic.SetScalarParameterValue` (`/Game/BP_GameManager.MI` (`self.GameManager`)) "Blend" (`KismetMathLibrary.FInterpEaseInOut` _returnvalue 2.0 _alpha_3 2.0))
              (set `/Game/BP_GameManager.LIghtMinValue` 0.4 (`self.GameManager`)))))
        (:`4`
          (bind (_direction_4 _alpha_4) (`Timeline|Timeline_1` :!via `PlayFromStart`)
            (:`Update`
              (`MaterialInstanceDynamic.SetScalarParameterValue` (`/Game/BP_GameManager.MI` (`self.GameManager`)) "Blend" (`KismetMathLibrary.FInterpEaseInOut` _returnvalue 4.0 _alpha_4 2.0))
              (set `/Game/BP_GameManager.LIghtMinValue` 0.2 (`self.GameManager`)))))
        (:`5`
          (bind (_direction_5 _sine) (`Timeline|Timeline_2` :!via `PlayFromStart`)
            (:`Update`
              (`MaterialInstanceDynamic.SetScalarParameterValue` (`/Game/BP_GameManager.MI` (`self.GameManager`)) "Blend" (* (`KismetMathLibrary.DegSin` (* _sine 100.0)) (`self.Amplitude`))))))
        (:`6`
          (bind (_direction_6 _alpha_5) (`Timeline|Timeline_3` :!via `PlayFromStart`)
            (:`Update`
              (set `self.Amplitude` (`KismetMathLibrary.FInterpEaseInOut` (`self.Amplitude`) 0.0 _alpha_5 1.0))
              (`/Engine/EditorBlueprintResources/StandardMacros.IsValid` _firstpersonchar
                (:`Is Valid`
                  (`/Game/FirstPerson/Blueprints/BP_FirstPersonCharacter.FadeCamera` _firstpersonchar))))))))))

(event `self.ReceiveTick`
  (params (DeltaSeconds :type "Float (single-precision)")))

(fn `UserConstructionScript`)