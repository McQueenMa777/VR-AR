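; Cube actor that toggles between dissolved and visible when the VR pawn registers a hit.
; BeginPlay caches the first VRPawn and creates a dynamic material instance on its mesh.
; Tick polls the pawn's Hit flag, prints a debug message, and triggers the dissolve behind a two-second lockout.
; Two timelines, chosen by a Visible flag, drive the material's Dissolve parameter out and back.
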(event `self.ReceiveBeginPlay`
  (bind _staticmeshcomponent (`self.StaticMeshComponent`))
  (bind _returnvalue (`GameplayStatics.GetActorOfClass` "/Game/VRTemplate/Blueprints/VRPawn.VRPawn_C"))
  (set `self.Char` _returnvalue)
  (bind _returnvalue_2 (`PrimitiveComponent.CreateDynamicMaterialInstance` _staticmeshcomponent 0 (`PrimitiveComponent.GetMaterial` _staticmeshcomponent 0) "None"))
  (set `self.DissolveMat` _returnvalue_2)
  (set `self.Visible` true))

(event `self.ReceiveTick`
  (params (DeltaSeconds :type "Float (single-precision)"))
  (if (`/Game/VRTemplate/Blueprints/VRPawn.Hit?` (`self.Char`))
    (if true
      (`KismetSystemLibrary.PrintString` "Hit" true true (struct :`R` 1.0 :`B` 0.155215 :`A` 1.0))
      (if (not (`self.triggered`))
        (set `self.triggered` true)
        (`self.dissolve`)
        (`KismetSystemLibrary.Delay` 2.0)
        (set `self.triggered` false)))))

(event `dissolve`
  (if (`self.Visible`)
    (bind (_direction _dissolve) (`Timeline|Timeline`)
      (:`Update`
        (`MaterialInstanceDynamic.SetScalarParameterValue` (`self.DissolveMat`) "Dissolve" _dissolve)
        (set `self.Visible` false)))
    (else
      (bind (_direction_2 _dissolverev) (`Timeline|Timeline_0`)
        (:`Update`
          (`MaterialInstanceDynamic.SetScalarParameterValue` (`self.DissolveMat`) "Dissolve" _dissolverev)
          (set `self.Visible` true))))))

(fn `UserConstructionScript`)