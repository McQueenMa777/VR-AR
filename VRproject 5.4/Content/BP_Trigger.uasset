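; BP_Trigger is a one-shot overlap trigger that advances a staged, increasingly creepy atmosphere through a counter on BP_GameManager.
; The count selects a timeline driving the manager's material "Blend" parameter.
; Stages one to four raise Blend and lower minimum light, with stage two also triggering a boat collision.
; Stage five adds audio and oscillates Blend until stage six, which eases it to zero and fades the VR camera.
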(event `self.ReceiveBeginPlay`
  (bind _returnvalue (`GameplayStatics.GetActorOfClass` "/Game/BP_GameManager.BP_GameManager_C"))
  (set `self.GameManager` _returnvalue)
  (bind _returnvalue_2 (`GameplayStatics.GetActorOfClass` "/Game/FirstPerson/Blueprints/BP_FirstPersonCharacter.BP_FirstPersonCharacter_C"))
  (set `self.FirstPersonChar` _returnvalue_2)
  (bind _returnvalue_3 (`GameplayStatics.GetActorOfClass` "/Game/VRTemplate/Blueprints/VRPawn.VRPawn_C"))
  (set `self.VRChar` _returnvalue_3))

(event `self.ReceiveActorBeginOverlap`
  (params (OtherActor :type "Actor Object Reference"))
  (bind _gamemanager (`self.GameManager`))
  (`/Engine/EditorBlueprintResources/StandardMacros.DoOnce` false
    (:`Completed`
      (bind _output_get (set `/Game/BP_GameManager.Triggers` (+ (`/Game/BP_GameManager.Triggers` _gamemanager) 1.0) _gamemanager))
      (bind _returnvalue (`MaterialInstanceDynamic.K2_GetScalarParameterValue` (`/Game/BP_GameManager.MI` (`self.GameManager`)) "Blend"))
      (switch `int` (`KismetMathLibrary.FTrunc` _output_get)
        (:`1`
          (bind (_direction _alpha) (`Timeline|Transition` :!via `PlayFromStart`)
            (:`Update`
              (`MaterialInstanceDynamic.SetScalarParameterValue` (`/Game/BP_GameManager.MI` (`self.GameManager`)) "Blend" (`KismetMathLibrary.FInterpEaseInOut` _returnvalue 0.2 _alpha 2.0))
              (set `/Game/BP_GameManager.LIghtMinValue` 0.8 (`self.GameManager`)))))
        (:`2`
          (bind _returnvalue_2 (`GameplayStatics.GetActorOfClass` "/Game/BPBoat.BPBoat_C"))
          (`/Game/BPBoat.BoatCollide` _returnvalue_2)
          (bind (_direction_2 _alpha_2) (`Timeline|Timeline` :!via `PlayFromStart`)
            (:`Update`
              (`MaterialInstanceDynamic.SetScalarParameterValue` (`/Game/BP_GameManager.MI` (`self.GameManager`)) "Blend" (`KismetMathLibrary.FInterpEaseInOut` _returnvalue 0.4 _alpha_2 2.0))
              (set `/Game/BP_GameManager.LIghtMinValue` 0.6 (`self.GameManager`)))))
        (:`3`
          (bind (_direction_3 _alpha_3) (`Timeline|Timeline_0` :!via `PlayFromStart`)
            (:`Update`
              (`MaterialInstanceDynamic.SetScalarParameterValue` (`/Game/BP_GameManager.MI` (`self.GameManager`)) "Blend" (`KismetMathLibrary.FInterpEaseInOut` _returnvalue 0.6 _alpha_3 2.0))
              (set `/Game/BP_GameManager.LIghtMinValue` 0.4 (`self.GameManager`)))))
        (:`4`
          (bind (_direction_4 _alpha_4) (`Timeline|Timeline_1` :!via `PlayFromStart`)
            (:`Update`
              (`MaterialInstanceDynamic.SetScalarParameterValue` (`/Game/BP_GameManager.MI` (`self.GameManager`)) "Blend" (`KismetMathLibrary.FInterpEaseInOut` _returnvalue 0.8 _alpha_4 2.0))
              (set `/Game/BP_GameManager.LIghtMinValue` 0.2 (`self.GameManager`)))))
        (:`5`
          (bind _returnvalue_3 (`AddComponent|NODE_AddAudioComponent-0`))
          (set `self.CreepySound` _returnvalue_3)
          (bind (_direction_5 _sine) (`Timeline|Timeline_2` :!via `PlayFromStart` :!label _label)
            (:`Update`
              (`MaterialInstanceDynamic.SetScalarParameterValue` (`/Game/BP_GameManager.MI` (`self.GameManager`)) "Blend" (`KismetMathLibrary.DegSin` (* _sine 100.0)))
              (if (== (`/Game/BP_GameManager.Triggers` (`self.GameManager`)) 6.0)
                (goto _label :!via `Stop`)))))
        (:`6`
          (bind _returnvalue_4 (`MaterialInstanceDynamic.K2_GetScalarParameterValue` (`/Game/BP_GameManager.MI` (`self.GameManager`)) "Blend"))
          (bind (_direction_6 _alpha_5) (`Timeline|Timeline_3` :!via `PlayFromStart`)
            (:`Update`
              (`|ExecutionSequence`
                (:`then_0`
                  (`MaterialInstanceDynamic.SetScalarParameterValue` (`/Game/BP_GameManager.MI` (`self.GameManager`)) "Blend" (`KismetMathLibrary.FInterpEaseInOut` _returnvalue_4 0.0 _alpha_5 1.0)))
                (:`then_1`
                  (`/Engine/EditorBlueprintResources/StandardMacros.DoOnce` false
                    (:`Completed`
                      (`/Game/VRTemplate/Blueprints/VRPawn.FadeCamera` (`self.VRChar`)))))))))))))

(fn `UserConstructionScript`)