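; A statue actor that slowly turns to keep facing the first-person player character.
; On BeginPlay it finds and caches the BP_FirstPersonCharacter.
; Each tick, while that reference is valid, it interpolates the Scene component toward a look-at rotation with a 90-degree yaw offset.
; Only the resulting yaw is applied, with pitch and roll held at zero so the statue stays upright.
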(event `self.ReceiveBeginPlay`
  (bind _returnvalue (`GameplayStatics.GetActorOfClass` "/Game/FirstPerson/Blueprints/BP_FirstPersonCharacter.BP_FirstPersonCharacter_C"))
  (set `self.FpChar` _returnvalue))

(event `self.ReceiveTick`
  (params (DeltaSeconds :type "Float (single-precision)"))
  (bind (_returnvalue_roll _returnvalue_pitch _returnvalue_yaw) (`KismetMathLibrary.BreakRotator` (`KismetMathLibrary.FindLookAtRotation` (`SceneComponent.K2_GetComponentLocation` (`self.Scene`)) (`self.K2_GetActorLocation` (`self.FpChar`)))))
  (bind (_returnvalue_roll_2 _returnvalue_pitch_2 _returnvalue_yaw_2) (`KismetMathLibrary.BreakRotator` (`KismetMathLibrary.RInterpTo` (`SceneComponent.K2_GetComponentRotation` (`self.Scene`)) (`KismetMathLibrary.MakeRotator` _returnvalue_roll _returnvalue_pitch (+ _returnvalue_yaw 90.0)) (`GameplayStatics.GetWorldDeltaSeconds`) 1.0)))
  (`/Engine/EditorBlueprintResources/StandardMacros.IsValid` (`self.FpChar`)
    (:`Is Valid`
      (`SceneComponent.K2_SetWorldRotation` (`self.Scene`) (`KismetMathLibrary.MakeRotator` 0.0 0.0 _returnvalue_yaw_2) false false))))

(fn `UserConstructionScript`)