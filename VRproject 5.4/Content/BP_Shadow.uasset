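; BP_Shadow is a short-lived shadow figure actor that plays one random animation, then dissolves and destroys itself.
; On BeginPlay it creates dynamic instances of its two mesh materials and picks a random non-looping clip from AnimToPlay.
; The chosen index starts a matching timeline that drives the Dissolve parameter on both materials and destroys the actor when finished.
; An unconnected random montage call never runs.
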(event `self.ReceiveBeginPlay`
  (bind _animtoplay (`self.AnimToPlay`))
  (bind _returnvalue (`PrimitiveComponent.CreateDynamicMaterialInstance` (`self.Mesh`) 0 "/Game/M_Shadow.M_Shadow" "None"))
  (set `self.M0` _returnvalue)
  (bind _returnvalue_2 (`PrimitiveComponent.CreateDynamicMaterialInstance` (`self.Mesh`) 1 "/Game/M_Shadow_Inst1.M_Shadow_Inst1" "None"))
  (set `self.M1` _returnvalue_2)
  (bind _output_get (set `self.RandomIndex` (`KismetMathLibrary.RandomInteger` (`KismetArrayLibrary.Array_Length` _animtoplay))))
  (`SkeletalMeshComponent.PlayAnimation` (`self.Mesh`) (`|GetArrayItem` _animtoplay _output_get) false)
  (switch `int` _output_get
    (:`0`
      (`KismetSystemLibrary.PrintString` "crawl")
      (bind (_direction _dissolve) (`Timeline|CrawlDissolve` :!via `PlayFromStart`)
        (:`Update`
          (`MaterialInstanceDynamic.SetScalarParameterValue` (`self.M0`) "Dissolve" _dissolve)
          (`MaterialInstanceDynamic.SetScalarParameterValue` (`self.M1`) "Dissolve" _dissolve))
        (:`Finished`
          (`self.K2_DestroyActor`))))
    (:`1`
      (`KismetSystemLibrary.PrintString` "exaggerated")
      (bind (_direction_2 _dissolve_2) (`Timeline|ExDissolve` :!via `PlayFromStart`)
        (:`Update`
          (`MaterialInstanceDynamic.SetScalarParameterValue` (`self.M0`) "Dissolve" _dissolve_2)
          (`MaterialInstanceDynamic.SetScalarParameterValue` (`self.M1`) "Dissolve" _dissolve_2))
        (:`Finished`
          (`self.K2_DestroyActor`))))
    (:`2`
      (`KismetSystemLibrary.PrintString` "look")
      (bind (_direction_3 _dissolve_3) (`Timeline|NPCdissolve` :!via `PlayFromStart`)
        (:`Update`
          (`MaterialInstanceDynamic.SetScalarParameterValue` (`self.M0`) "Dissolve" _dissolve_3)
          (`MaterialInstanceDynamic.SetScalarParameterValue` (`self.M1`) "Dissolve" _dissolve_3))
        (:`Finished`
          (`self.K2_DestroyActor`))))
    (:`3`
      (`KismetSystemLibrary.PrintString` "oldman")
      (bind (_direction_4 _dissolve_4) (`Timeline|OldDissolve` :!via `PlayFromStart`)
        (:`Update`
          (`MaterialInstanceDynamic.SetScalarParameterValue` (`self.M0`) "Dissolve" _dissolve_4)
          (`MaterialInstanceDynamic.SetScalarParameterValue` (`self.M1`) "Dissolve" _dissolve_4))
        (:`Finished`
          (`self.K2_DestroyActor`))))
    (:`4`
      (`KismetSystemLibrary.PrintString` "reception")
      (bind (_direction_5 _dissolve_5) (`Timeline|RecepDissolve` :!via `PlayFromStart`)
        (:`Update`
          (`MaterialInstanceDynamic.SetScalarParameterValue` (`self.M0`) "Dissolve" _dissolve_5)
          (`MaterialInstanceDynamic.SetScalarParameterValue` (`self.M1`) "Dissolve" _dissolve_5))
        (:`Finished`
          (`self.K2_DestroyActor`))))
    (:`5`
      (`KismetSystemLibrary.PrintString` "wall")
      (bind (_direction_6 _dissolve_6) (`Timeline|ClimbDissolve` :!via `PlayFromStart`)
        (:`Update`
          (`MaterialInstanceDynamic.SetScalarParameterValue` (`self.M0`) "Dissolve" _dissolve_6)
          (`MaterialInstanceDynamic.SetScalarParameterValue` (`self.M1`) "Dissolve" _dissolve_6))
        (:`Finished`
          (`self.K2_DestroyActor`))))
    (:`6`
      (`KismetSystemLibrary.PrintString` "walking")
      (bind (_direction_7 _dissolve_7) (`Timeline|Walk` :!via `PlayFromStart`)
        (:`Update`
          (`MaterialInstanceDynamic.SetScalarParameterValue` (`self.M0`) "Dissolve" _dissolve_7)
          (`MaterialInstanceDynamic.SetScalarParameterValue` (`self.M1`) "Dissolve" _dissolve_7))
        (:`Finished`
          (`self.K2_DestroyActor`))))))

(fn `UserConstructionScript`)