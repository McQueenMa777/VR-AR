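; BP_LIght is a Blueprint that makes its point light flicker erratically from BeginPlay onward.
; Each Flicker call randomly switches the light either off or to a random intensity within a bright range.
; Flicker then clears and re-arms its own timer by function name with a short random delay, producing an irregular, self-rescheduling loop without Tick.
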(event `self.ReceiveBeginPlay`
  (`KismetSystemLibrary.K2_SetTimer` null "Flicker" 0.1))

(event `Flicker`
  (`LightComponent.SetIntensity` (`self.PointLight`) (`|GetArrayItem` (`|MakeArray` (`KismetMathLibrary.RandomFloatInRange` 1000.0 3000.0) 0.0) (`KismetMathLibrary.RandomIntegerInRange` 0 1)))
  (`KismetSystemLibrary.K2_ClearTimer` null "Flicker")
  (bind _output_get (set `self.Delay` (`KismetMathLibrary.RandomFloatInRange` 0.1 0.5)))
  (`KismetSystemLibrary.K2_SetTimer` null "Flicker" _output_get))

(fn `UserConstructionScript`)