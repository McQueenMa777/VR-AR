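; BP_Paint is a painting that turns into a video when the first-person character's hit name reads "frame".
; BeginPlay caches the character and applies the painting material, then Tick polls that hit name while no video is playing.
; Play swaps the mesh to the media material and opens the video source, and the end-reached callback restores the painting and clears the playing flag.
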(event `self.ReceiveBeginPlay`
  (bind _returnvalue (`GameplayStatics.GetActorOfClass` "/Game/FirstPerson/Blueprints/BP_FirstPersonCharacter.BP_FirstPersonCharacter_C"))
  (set `self.Character` _returnvalue)
  (`PrimitiveComponent.SetMaterial` (`self.StaticMeshComponent`) 0 "/Game/VRModel/Frame/M_Painting.M_Painting"))

(event `self.ReceiveTick`
  (params (DeltaSeconds :type "Float (single-precision)"))
  (if (`KismetStringLibrary.EqualEqual_StrStr` (`/Game/FirstPerson/Blueprints/BP_FirstPersonCharacter.Hitname` (`self.Character`)) "frame")
    (if (not (`self.Playing`))
      (`self.Play`))))

(event `Play`
  (bind _player (`self.Player`))
  (set `self.Playing` true)
  (`PrimitiveComponent.SetMaterial` (`self.StaticMeshComponent`) 0 "/Game/VRModel/FrameTexture/NewMediaPlayer_Video_Mat.NewMediaPlayer_Video_Mat")
  (`MediaPlayer.OpenSource` _player "/Game/VRModel/FrameTexture/PaintVideo.PaintVideo")
  (add `MediaPlayer.OnEndReached` _player (delegate `OnEndReached_Event`)))

(event `OnEndReached_Event`
  (`PrimitiveComponent.SetMaterial` (`self.StaticMeshComponent`) 0 "/Game/VRModel/Frame/M_Painting.M_Painting")
  (set `self.Playing` false))

(fn `UserConstructionScript`)